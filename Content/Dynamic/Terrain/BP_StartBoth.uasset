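; BP_StartBoth is a terrain barrier actor that plays a sound at BeginPlay and responds only to player character 0.
; Entering LockingVolume unlocks it and leaving relocks it, swapping the barrier's collision object type and its green or red material.
; Switching between two custom collision channels changes what the barrier blocks without toggling collision.
; Overlapping DestroyVolume destroys the whole actor.
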(event `self.ReceiveBeginPlay`
  (`GameplayStatics.SpawnSoundAtLocation` "/Game/Dynamic/Sounds/Terrain/Tile/Cue_Barrier_Sound.Cue_Barrier_Sound" (`SceneComponent.K2_GetComponentLocation` (`self.Barrier`))))

(event `self.LockingVolume.OnComponentBeginOverlap`
  (params (OverlappedComponent :type "PrimitiveComponent Object Reference") (OtherActor :type "Actor Object Reference") (OtherComp :type "PrimitiveComponent Object Reference") (OtherBodyIndex :type Integer) (bFromSweep :type Boolean) (SweepResult :type "HitResult Structure (by ref)"))
  (`self.IsPlayer` OtherActor)
  (`self.UnLock`))

(event `self.LockingVolume.OnComponentEndOverlap`
  (params (OverlappedComponent :type "PrimitiveComponent Object Reference") (OtherActor :type "Actor Object Reference") (OtherComp :type "PrimitiveComponent Object Reference") (OtherBodyIndex :type Integer))
  (`self.IsPlayer` OtherActor)
  (`self.Lock`))

(event `self.DestroyVolume.OnComponentBeginOverlap`
  (params (OverlappedComponent :type "PrimitiveComponent Object Reference") (OtherActor :type "Actor Object Reference") (OtherComp :type "PrimitiveComponent Object Reference") (OtherBodyIndex :type Integer) (bFromSweep :type Boolean) (SweepResult :type "HitResult Structure (by ref)"))
  (`self.IsPlayer` OtherActor)
  (`self.K2_DestroyActor`))

(fn `Lock`
  (bind _barrier (`self.Barrier`))
  (`PrimitiveComponent.SetCollisionObjectType` _barrier "ECC_GameTraceChannel6")
  (`PrimitiveComponent.SetMaterial` _barrier 0 "/Game/Static/Terrain/Materials/Materials/MI_Barrier_Red.MI_Barrier_Red"))

(fn `UnLock`
  (bind _barrier (`self.Barrier`))
  (`PrimitiveComponent.SetCollisionObjectType` _barrier "ECC_GameTraceChannel7")
  (`PrimitiveComponent.SetMaterial` _barrier 0 "/Game/Static/Terrain/Materials/Materials/MI_Barrier_Green.MI_Barrier_Green"))

(fn `UserConstructionScript`)