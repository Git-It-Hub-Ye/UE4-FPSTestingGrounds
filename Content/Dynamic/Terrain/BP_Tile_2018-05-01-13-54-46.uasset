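; Terrain tile for an infinite-terrain mode that randomly populates itself on BeginPlay with AI bots, cover props, rocks and pickups.
; Its barrier starts locked; the player overlapping LockingVolume switches its collision channel and red/green material, and first entry reports the tile conquered to the game mode.
; Player overlap with DestroyVolume has the game mode spawn another tile and destroys this one, while DestroyBox reopens TileMap.
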(event `self.ReceiveBeginPlay`
  (`self.Lock`)
  (`self.PlaceAIPawns` "/Game/Dynamic/Character/Behaviour/BP_AIBot.BP_AIBot_C" (make `SpawnParameters` (`self.MinEnimies`) (`self.MaxEnimies`) 100))
  (`self.PlaceActors` "/Game/Dynamic/Terrain/Props/BP_Container.BP_Container_C" (make `SpawnParameters` 1 4))
  (`self.PlaceActors` "/Game/Dynamic/Terrain/Props/BP_SandBags.BP_SandBags_C" (make `SpawnParameters` 1 3 300))
  (`self.PlaceActors` "/Game/Dynamic/Terrain/Props/BP_Box.BP_Box_C" (make `SpawnParameters` 4 6 100))
  (`self.PlaceActors` "/Game/Dynamic/Terrain/Props/BP_Rock02.BP_Rock02_C" (make `SpawnParameters` 1 2 280 1.0 2.0))
  (`self.PlaceActors` "/Game/Dynamic/Terrain/Props/BP_Rock01.BP_Rock01_C" (make `SpawnParameters` 1 2 160 1.0 2.5))
  (`self.PlaceActors` "/Game/Dynamic/Terrain/Props/BP_Canister.BP_Canister_C" (make `SpawnParameters` 2 5 100))
  (`self.PlaceActors` "/Game/Dynamic/Terrain/Props/BP_Rock03.BP_Rock03_C" (make `SpawnParameters` 1 2 250 1.0 1.6))
  (`self.PlaceActors` "/Game/Dynamic/PickUps/BP_PickUp_Ammo_GrenadeLauncher.BP_PickUp_Ammo_GrenadeLauncher_C" (make `SpawnParameters` 0 1 100))
  (`self.PlaceActors` "/Game/Dynamic/PickUps/BP_PickUp_Ammo_ShotGun.BP_PickUp_Ammo_ShotGun_C" (make `SpawnParameters` 0 1 100))
  (`self.PlaceActors` "/Game/Dynamic/PickUps/BP_PickUp_Health.BP_PickUp_Health_C" (make `SpawnParameters` 0 2 100))
  (`GameplayStatics.SpawnSoundAtLocation` "/Game/Dynamic/Sounds/Terrain/Tile/Cue_Barrier_Sound.Cue_Barrier_Sound" (`SceneComponent.K2_GetComponentLocation` (`self.Barrier`))))

(event `self.LockingVolume.OnComponentBeginOverlap`
  (params (OverlappedComponent :type "PrimitiveComponent Object Reference") (OtherActor :type "Actor Object Reference") (OtherComp :type "PrimitiveComponent Object Reference") (OtherBodyIndex :type Integer) (bFromSweep :type Boolean) (SweepResult :type "HitResult Structure (by ref)"))
  (`self.Is Player` OtherActor)
  (`|ExecutionSequence`
    (:`then_0`
      (`self.Unlock`))
    (:`then_1`
      (`self.NewTileConquered`))))

(event `self.LockingVolume.OnComponentEndOverlap`
  (params (OverlappedComponent :type "PrimitiveComponent Object Reference") (OtherActor :type "Actor Object Reference") (OtherComp :type "PrimitiveComponent Object Reference") (OtherBodyIndex :type Integer))
  (`self.Is Player` OtherActor)
  (`self.Lock`))

(event `self.DestroyVolume.OnComponentBeginOverlap`
  (params (OverlappedComponent :type "PrimitiveComponent Object Reference") (OtherActor :type "Actor Object Reference") (OtherComp :type "PrimitiveComponent Object Reference") (OtherBodyIndex :type Integer) (bFromSweep :type Boolean) (SweepResult :type "HitResult Structure (by ref)"))
  (`self.Is Player` OtherActor)
  (bind _asbp_infinite_terrain_game_mode (cast `/Game/Dynamic/BP_InfiniteTerrainGameMode` (`GameplayStatics.GetGameMode`)))
  (`InfiniteTerrainGameMode.SpawnTile` _asbp_infinite_terrain_game_mode)
  (`self.K2_DestroyActor`))

(event `self.DestroyBox.OnComponentBeginOverlap`
  (params (OverlappedComponent :type "PrimitiveComponent Object Reference") (OtherActor :type "Actor Object Reference") (OtherComp :type "PrimitiveComponent Object Reference") (OtherBodyIndex :type Integer) (bFromSweep :type Boolean) (SweepResult :type "HitResult Structure (by ref)"))
  (bind _returnvalue (`GameplayStatics.GetPlayerController` 0))
  (`self.Is Player` OtherActor)
  (`GameplayStatics.OpenLevel` "TileMap")
  (set `PlayerController.bShowMouseCursor` false _returnvalue)
  (`WidgetBlueprintLibrary.SetInputMode_GameOnly` _returnvalue))

(fn `Lock`
  (bind _barrier (`self.Barrier`))
  (`PrimitiveComponent.SetCollisionObjectType` _barrier "ECC_GameTraceChannel6")
  (`PrimitiveComponent.SetMaterial` _barrier 0 "/Game/Static/Terrain/Materials/Materials/MI_Barrier_Red.MI_Barrier_Red"))

(fn `NewTileConquered`
  (if (not (`self.IsTileConquered`))
    (bind _asbp_infinite_terrain_game_mode (cast `/Game/Dynamic/BP_InfiniteTerrainGameMode` (`GameplayStatics.GetGameMode`)))
    (`InfiniteTerrainGameMode.PlayerConqueredTile` _asbp_infinite_terrain_game_mode)
    (set `self.IsTileConquered` true)
    (`GameplayStatics.SpawnSound2D` "/Game/Dynamic/Sounds/Terrain/Tile/Cue_EnterTile.Cue_EnterTile")))

(fn `Unlock`
  (bind _barrier (`self.Barrier`))
  (`PrimitiveComponent.SetCollisionObjectType` _barrier "ECC_GameTraceChannel7")
  (`PrimitiveComponent.SetMaterial` _barrier 0 "/Game/Static/Terrain/Materials/Materials/MI_Barrier_Green.MI_Barrier_Green"))

(fn `UserConstructionScript`)