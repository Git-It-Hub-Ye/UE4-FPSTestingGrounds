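; BP_Tile_Menu is a terrain tile with a lockable barrier that reports to the infinite terrain game mode when conquered.
; It starts locked with a barrier sound; Lock and Unlock swap the barrier's collision object type and red or green material.
; NewTileConquered fires once, notifying the game mode and playing an entry sound.
; An Is Player helper compares an actor to the player character, and nothing here calls Unlock or NewTileConquered.
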(event `self.ReceiveBeginPlay`
  (`self.Lock`)
  (`GameplayStatics.SpawnSoundAtLocation` "/Game/Dynamic/Sounds/Terrain/Tile/Cue_Barrier_Sound.Cue_Barrier_Sound" (`SceneComponent.K2_GetComponentLocation` (`self.Barrier`))))

(fn `Lock`
  (bind _barrier (`self.Barrier`))
  (`PrimitiveComponent.SetCollisionObjectType` _barrier "ECC_GameTraceChannel6")
  (`PrimitiveComponent.SetMaterial` _barrier 0 "/Game/Static/Terrain/Materials/Materials/MI_Barrier_Red.MI_Barrier_Red"))

(fn `NewTileConquered`
  (if (not (`self.IsTileConquered`))
    (bind _asbp_infinite_terrain_game_mode (cast `/Game/Dynamic/Blueprints/BP_InfiniteTerrainGameMode` (`GameplayStatics.GetGameMode`)))
    (`InfiniteTerrainGameMode.PlayerConqueredTile` _asbp_infinite_terrain_game_mode)
    (set `self.IsTileConquered` true)
    (`GameplayStatics.SpawnSound2D` "/Game/Dynamic/Sounds/Terrain/Tile/Cue_EnterTile.Cue_EnterTile")))

(fn `Unlock`
  (bind _barrier (`self.Barrier`))
  (`PrimitiveComponent.SetCollisionObjectType` _barrier "ECC_GameTraceChannel7")
  (`PrimitiveComponent.SetMaterial` _barrier 0 "/Game/Static/Terrain/Materials/Materials/MI_Barrier_Green.MI_Barrier_Green"))

(fn `UserConstructionScript`)