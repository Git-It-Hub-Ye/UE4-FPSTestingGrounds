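; BP_StartBoth_Menu is a terrain barrier actor, apparently for the menu, that switches between locked and unlocked states.
; Lock and UnLock swap the Barrier component's collision object channel and its red or green material.
; On BeginPlay it unlocks itself and spawns a barrier sound at the Barrier's location.
; An IsPlayer graph compares an actor to the first player character, but nothing shown here calls it or Lock.
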(event `self.ReceiveBeginPlay`
  (`self.UnLock`)
  (`GameplayStatics.SpawnSoundAtLocation` "/Game/Dynamic/Sounds/Terrain/Tile/Cue_Barrier_Sound.Cue_Barrier_Sound" (`SceneComponent.K2_GetComponentLocation` (`self.Barrier`))))

(fn `Lock`
  (bind _barrier (`self.Barrier`))
  (`PrimitiveComponent.SetCollisionObjectType` _barrier "ECC_GameTraceChannel6")
  (`PrimitiveComponent.SetMaterial` _barrier 0 "/Game/Static/Terrain/Materials/Materials/MI_Barrier_Red.MI_Barrier_Red"))

(fn `UnLock`
  (bind _barrier (`self.Barrier`))
  (`PrimitiveComponent.SetCollisionObjectType` _barrier "ECC_GameTraceChannel7")
  (`PrimitiveComponent.SetMaterial` _barrier 0 "/Game/Static/Terrain/Materials/Materials/MI_Barrier_Green.MI_Barrier_Green"))

(fn `UserConstructionScript`)